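; BP_SpeedBoost is a pickup actor that temporarily raises the player's forward speed.
; When BP_Player overlaps it, the cube mesh is hidden and the player's ForwardForce is doubled.
; After a short delay the force is set back to a hard-coded normal value and the actor destroys itself.
; Collision stays active during the delay, as only the mesh visibility changes.
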(event `self.ReceiveActorBeginOverlap`
  (params (OtherActor :type "Actor Object Reference"))
  (bind _asbp_player (cast `/Game/BlockHead/Core/Actors/BP_Player` OtherActor))
  (set `self.Player` _asbp_player)
  (`|ExecutionSequence`
    (:`then_0`
      (`SceneComponent.SetVisibility` (`self.Cube`) false false))
    (:`then_1`
      (set `/Game/BlockHead/Core/Actors/BP_Player.ForwardForce` 2000.0 (`self.Player`))
      (`KismetSystemLibrary.Delay` 3.0)
      (set `/Game/BlockHead/Core/Actors/BP_Player.ForwardForce` 1000.0 (`self.Player`))
      (`self.K2_DestroyActor`))))

(fn `UserConstructionScript`)